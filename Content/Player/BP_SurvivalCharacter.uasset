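; Player character for a survival game, with Enhanced Input movement, look, hold-to-sprint, resource harvesting and basic survival stats.
; Interact line-traces from the camera to BP_ResourceBase actors, spending stamina to leave a hit decal and add wood, stone or berries.
; Each harvest depletes the resource, which is hidden with collision disabled when empty.
; A looping timer drives stat updates: hunger drains, health drops while starving, and stamina regenerates.
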(event Custom|UpdatePlayerStats
  ;[0.15 0.15 0.15 0.5] Hunger&Health
  (Variables|PlayerStats|SetHunger (Math|Float|Clamp(Float) (- (Variables|PlayerStats|GetHunger) 1.0) 0.0 1e+02))
  (if (<= (Variables|PlayerStats|GetHunger) 0.0)
    (Variables|PlayerStats|SetHealth (Math|Float|Clamp(Float) (- (Variables|PlayerStats|GetHealth) 1.0) 0.0 1e+02)))
  (Variables|PlayerStats|SetStamina (Math|Float|Clamp(Float) (+ (Variables|PlayerStats|GetStamina) 1.0) 0.0 1e+02)))

(event Input|EnhancedActionEvents|EnhancedInputActionIA_Move
  (params (ActionValue :type Vector%202D%20Structure) (ElapsedSeconds :type Float%20%28double-precision%29) (TriggeredSeconds :type Float%20%28double-precision%29) (InputAction :type Input%20Action%20Object%20Reference :default "/Game/Player/IA_Move.IA_Move"))
  ;[0.15 0.15 0.15 0.5] Keyboard
  (Pawn|Input|AddMovementInput (Transformation|GetActorForwardVector) (.y ActionValue) false)
  (Pawn|Input|AddMovementInput (Transformation|GetActorRightVector) (.x ActionValue) false))

(event Input|EnhancedActionEvents|EnhancedInputActionIA_Look
  (params (ActionValue :type Vector%202D%20Structure) (ElapsedSeconds :type Float%20%28double-precision%29) (TriggeredSeconds :type Float%20%28double-precision%29) (InputAction :type Input%20Action%20Object%20Reference :default "/Game/Player/IA_Look.IA_Look"))
  ;[0.15 0.15 0.15 0.5] Mouse
  (Pawn|Input|AddControllerYawInput (.x ActionValue))
  (Pawn|Input|AddControllerPitchInput (.y ActionValue)))

(event Input|EnhancedActionEvents|EnhancedInputActionIA_Sprint
  (params (ActionValue :type Boolean) (ElapsedSeconds :type Float%20%28double-precision%29) (TriggeredSeconds :type Float%20%28double-precision%29) (InputAction :type Input%20Action%20Object%20Reference :default "/Game/Player/IA_Sprint.IA_Sprint"))
  (bind _charactermovement (Variables|Character|GetCharacterMovement))
  ;[0.15 0.15 0.15 0.5] Hold Left Shift to sprint; release it to restore walking speed to 300
  (:Started
    (Variables|/Script/Engine.CharacterMovementComponent|SetMaxWalkSpeed _charactermovement 1.2e+03))
  (:Canceled
    (Variables|/Script/Engine.CharacterMovementComponent|SetMaxWalkSpeed _charactermovement 3e+02 :!label _label))
  (:Completed
    (goto _label)))

(event Input|EnhancedActionEvents|EnhancedInputActionIA_Interact
  (params (ActionValue :type Boolean) (ElapsedSeconds :type Float%20%28double-precision%29) (TriggeredSeconds :type Float%20%28double-precision%29) (InputAction :type Input%20Action%20Object%20Reference :default "/Game/Player/IA_Interact.IA_Interact"))
  (bind _playercamera (Variables|Default|GetPlayerCamera))
  (bind _returnvalue (Transformation|GetWorldLocation _playercamera))
  ;[0.15 0.15 0.15 0.5] Resource harvesting and stamina cost
  (:Started
    (bind _outhit (Collision|LineTraceByChannel _returnvalue (+ _returnvalue (* (Math|Vector|GetForwardVector _playercamera) "500.000000,500.000000,500.000000")) "TraceTypeQuery1" false 0 "None"))
    (Utilities|IsValid (.HitActor (Collision|BreakHitResult _outhit))
      (:Is%20Valid
        (bind _asbp_resource_base (Utilities|Casting|CastToBP_ResourceBase (.HitActor (Collision|BreakHitResult _outhit))))
        (if (> (Variables|/Game/Resources/BP_ResourceBase.BP_ResourceBase_C|GetRemainingAmount _asbp_resource_base) 0)
          (if (> (Variables|PlayerStats|GetStamina) 5.0)
            (Variables|PlayerStats|SetStamina (- (Variables|PlayerStats|GetStamina) 5.0))
            (Rendering|Decal|SpawnDecalatLocation "/Game/Material/M_HitDecal.M_HitDecal" "64.000000,16.000000,16.000000" (.ImpactPoint (Collision|BreakHitResult _outhit)) (Math|Rotator|MakeRotfromX (.Normal (Collision|BreakHitResult _outhit))) 0.0)
            (switch name (Variables|/Game/Resources/BP_ResourceBase.BP_ResourceBase_C|GetResourceType _asbp_resource_base)
              (:Wood
                (Variables|Resources|SetWood (+ (Variables|Resources|GetWood) 1)))
              (:Stone
                (Variables|Resources|SetStone (+ (Variables|Resources|GetStone) 1)))
              (:Berry
                (Variables|Resources|SetBerry (+ (Variables|Resources|GetBerry) 1))))
            (bind _output_get (Variables|/Game/Resources/BP_ResourceBase.BP_ResourceBase_C|SetRemainingAmount _asbp_resource_base (- (stale _output_get) 1)))
            (if (<= _output_get 0)
              (Rendering|SetActorHiddenInGame _asbp_resource_base true)
              (Collision|SetActorEnableCollision _asbp_resource_base false))))))))

(event EventBeginPlay
  ;[0.15 0.15 0.15 0.5] Mouse and Keyboard
  (Utilities|Time|SetTimerbyEvent (EventDispatchers|CreateEvent :!event Custom|UpdatePlayerStats) 2.0 true)
  (Input|AddMappingContext (PlayerController|LocalPlayerSubsystems|GetEnhancedInputLocalPlayerSubsystem (Game|GetPlayerController 0)) "/Game/Player/IMC_Player.IMC_Player" 0 "(bIgnoreAllPressedKeysUntilRelease=True,bForceImmediately=False,bNotifyUserSettings=False)"))

(fn ConstructionScript)